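; BP_Doctor generates randomized doctor details, namely a name and a perk.
; RandomizeName picks a random row from DT_NpcInfoRandomizer for the name.
; RandomizePerk does the same with DT_DoctorRandomizer, returning the perk name, affected races, and positive and negative bonus descriptions.
; AddDoctor calls both functions in sequence but does not yet store or use their results.
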(fn `AddDoctor`
  (`self.RandomizeName`)
  (`self.RandomizePerk`))

(fn `RandomizeName`
  (returns (Name :type String))
  (bind _outrownames (`DataTableFunctionLibrary.GetDataTableRowNames` "/Game/Blueprints/AI/NPCData/DT_NpcInfoRandomizer.DT_NpcInfoRandomizer"))
  (bind _returnvalue (`|GetDataTableRow` "/Game/Blueprints/AI/NPCData/DT_NpcInfoRandomizer.DT_NpcInfoRandomizer" (`KismetArrayLibrary.Array_Random` _outrownames))
    (:`then`
      (return (`.Name_2_24B431884901098C891DEEBEC5213BD3` (break `/Game/Blueprints/AI/NPCData/S_NPCInfoRandomizer` _returnvalue))))))

(fn `RandomizePerk`
  (returns (PerkName :type String) (AffectedRaces :type "Array of /Game/Blueprints/AI/NPCData/E_Race Enum") (PositiveBonusDesc :type String) (NegativeBonusDesc :type String))
  (bind _outrownames (`DataTableFunctionLibrary.GetDataTableRowNames` "/Game/Blueprints/Doctors/PerksInfo/DT_DoctorRandomizer.DT_DoctorRandomizer"))
  (bind _returnvalue (`|GetDataTableRow` "/Game/Blueprints/Doctors/PerksInfo/DT_DoctorRandomizer.DT_DoctorRandomizer" (`KismetArrayLibrary.Array_Random` _outrownames))
    (:`then`
      (bind (_perkname _affectedrace _positivebonusdesc _negativebonusdesc) (break `/Game/Blueprints/Doctors/PerksInfo/S_DoctorRandomizer` _returnvalue))
      (return _perkname _affectedrace _positivebonusdesc _negativebonusdesc))))