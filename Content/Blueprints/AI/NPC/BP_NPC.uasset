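; BP_NPC is an NPC pawn that rolls a random identity and disease when play begins.
; It picks random rows from DT_NpcInfoRandomizer and DT_DiseaseRandomizer and only prints the name, age, race, disease, healing time and death chance, without storing them.
; A MoveTo event sends the pawn to a given actor with AIMoveTo and prints success or failure.
; An unconnected loop for visiting an array of destinations in sequence never runs.
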(event `MoveTo`
  (params (Destination :type "TargetPoint Object Reference"))
  (`|AIMoveTo` self (0.0 0.0 0.0) Destination
    (:`OnSuccess`
      (`KismetSystemLibrary.PrintString` "Success"))
    (:`OnFail`
      (`KismetSystemLibrary.PrintString` "Fail"))))

(event `self.ReceiveBeginPlay`
  (`self.RandomizeNPCInfo`)
  (`self.RandomizeDisease`))

(fn `RandomizeDisease`
  (bind _outrownames (`DataTableFunctionLibrary.GetDataTableRowNames` "/Game/Blueprints/AI/NPCData/DT_DiseaseRandomizer.DT_DiseaseRandomizer"))
  (bind _returnvalue (`|GetDataTableRow` "/Game/Blueprints/AI/NPCData/DT_DiseaseRandomizer.DT_DiseaseRandomizer" (`KismetArrayLibrary.Array_Random` _outrownames))
    (:`then`
      (bind (_disease _healingtime _deathchances) (break `/Game/Blueprints/AI/NPCData/S_DiseaseRandomizer` _returnvalue))
      (`KismetSystemLibrary.PrintText` (`|FormatText` "disease: {1} \nTime: {2} \ndeatch chance: {3}" (`|GetEnumeratorNameAsString` (cast `/Game/Blueprints/AI/NPCData/E_Diseases` _disease)) _healingtime _deathchances)))))

(fn `RandomizeNPCInfo`
  (bind _outrownames (`DataTableFunctionLibrary.GetDataTableRowNames` "/Game/Blueprints/AI/NPCData/DT_NpcInfoRandomizer.DT_NpcInfoRandomizer"))
  (bind _returnvalue (`|GetDataTableRow` "/Game/Blueprints/AI/NPCData/DT_NpcInfoRandomizer.DT_NpcInfoRandomizer" (`KismetArrayLibrary.Array_Random` _outrownames))
    (:`then`
      (bind (_name _age _race) (break `/Game/Blueprints/AI/NPCData/S_NPCInfoRandomizer` _returnvalue))
      (`KismetSystemLibrary.PrintText` (`|FormatText` "Name: {Name} \nAge: {Age} \nRace: {Race}" _name _age (`|GetEnumeratorNameAsString` (cast `/Game/Blueprints/AI/NPCData/E_Race` _race)))))))

(fn `UserConstructionScript`)