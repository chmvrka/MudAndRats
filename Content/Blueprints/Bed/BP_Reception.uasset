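; BP_Reception is a reception actor that sends arriving NPC patients to a free bed.
; When an actor overlaps its Collision, it stores that actor and scans the Beds array for the first free bed.
; SendPatientToBed moves the shared BedPointLocation target beside that bed and tells the BP_NPC to move to it.
; It never marks the bed occupied itself, and debug prints and spheres trace the process.
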(event `self.Collision.OnComponentBeginOverlap`
  (params (OverlappedComponent :type "PrimitiveComponent Object Reference") (OtherActor :type "Actor Object Reference") (OtherComp :type "PrimitiveComponent Object Reference") (OtherBodyIndex :type Integer) (bFromSweep :type Boolean) (SweepResult :type "HitResult Structure (by ref)"))
  (set `self.NPC` OtherActor)
  ; Checking if any bed is free
  (`KismetSystemLibrary.PrintString` "Hit Reception")
  (for _array_element (`self.Beds`)
    (`KismetSystemLibrary.PrintString` (`KismetSystemLibrary.GetDisplayName` _array_element))
    (if (`/Game/Blueprints/Bed/BP_Bed.IsFree?` _array_element)
      (`KismetSystemLibrary.PrintString` "Free")
      (set `self.FreeBed` _array_element)
      (set `self.IsFree?` true)
      (break)
      (else
        (`KismetSystemLibrary.PrintString` "Not Free"))))
  (`self.SendPatientToBed` (`self.FreeBed`)))

(event `SendPatientToBed`
  (params (WhichBed :type "/Game/Blueprints/Bed/BP_Bed Object Reference"))
  (bind _location (`/Game/Blueprints/Bed/BP_Bed.Location` WhichBed))
  (if (`/Game/Blueprints/Bed/BP_Bed.IsFree?` WhichBed)
    (bind _npc (`self.NPC`)
      (:`then`
        (set `self.IsFree?` true)
        (`KismetSystemLibrary.DrawDebugSphere` _location 100.0 12 (struct :`R` 1.0 :`G` 0.211459 :`A` 1.0) 1.0)
        (`KismetSystemLibrary.DrawDebugSphere` (`self.K2_GetActorLocation` _npc) 100.0 12 (struct :`R` 1.0 :`G` 0.211459 :`A` 1.0) 1.0)
        ; Set Bed Target Point for NPC
        (`KismetSystemLibrary.PrintString` "Break")
        (`SceneComponent.K2_SetWorldLocation` (`Actor.RootComponent` (`self.BedPointLocation`)) (+ _location (0.0 150.0 0.0)) false false)
        (bind _asbp_npc (cast `/Game/Blueprints/AI/NPC/BP_NPC` (`self.NPC`)))
        (`/Game/Blueprints/AI/NPC/BP_NPC.MoveTo` _asbp_npc (`self.BedPointLocation`))
        (set `self.NPC` null))
      (:`else`))))

(fn `UserConstructionScript`)