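; BP_Bed is a hospital bed actor that heals whatever actor overlaps its box, then frees itself for the next patient.
; On overlap it marks itself occupied and runs the HealingTime macro, a one-second Delay loop that shows the countdown on a 3D text.
; When the count reaches zero, it resets its state and timer, asks BP_Reception to send another patient, and destroys the healed actor.
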(event `self.ReceiveBeginPlay`
  (set `self.Location` (`self.K2_GetActorLocation`)))

(event `self.Box.OnComponentBeginOverlap`
  (params (OverlappedComponent :type "PrimitiveComponent Object Reference") (OtherActor :type "Actor Object Reference") (OtherComp :type "PrimitiveComponent Object Reference") (OtherBodyIndex :type Integer) (bFromSweep :type Boolean) (SweepResult :type "HitResult Structure (by ref)"))
  (set `self.IsFree?` false)
  (`self.HealingTime` (`self.Time`)
    (:`Out`
      (`self.PacientHealed`)
      (`self.K2_DestroyActor` OtherActor))))

(event `PacientHealed`
  (set `self.IsFree?` true)
  (set `self.Time` 5)
  (bind _returnvalue (`GameplayStatics.GetActorOfClass` "/Game/Blueprints/Bed/BP_Reception.BP_Reception_C"))
  (`/Game/Blueprints/Bed/BP_Reception.SendPatientToBed` _returnvalue self))

(fn `UserConstructionScript`)