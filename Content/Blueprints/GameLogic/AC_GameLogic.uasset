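; AC_GameLogic is a debug-key prototype for randomly picking E_WarChoices values, apparently for a War-style choice game.
; Key 1 runs a hand-wired counter loop that prints three random enum entries to the screen.
; Key 2 stores one random index from the RNG helper in Result1, then resets and increments the counter without looping, so that branch appears unfinished.
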(event `Key|One`
  (params (Key :type "Key Structure"))
  (:`Pressed`
    (set `self.LoopCounter` 0)
    (if (not (== (`self.LoopCounter`) 3)) :!label _label
      (`KismetSystemLibrary.PrintString` (`|GetEnumeratorNameAsString` (cast `/Game/Blueprints/GameLogic/E_WarChoices` (`KismetMathLibrary.Conv_IntToByte` (`KismetMathLibrary.RandomIntegerInRange` 0 (- (enumcount `/Game/Blueprints/GameLogic/E_WarChoices`) 1))))))
      (bind _result (`/Engine/EditorBlueprintResources/StandardMacros.IncrementInt` (`self.LoopCounter`))
        (:`  `
          (set `self.LoopCounter` _result)
          (goto _label))))))

(event `Key|Two`
  (params (Key :type "Key Structure"))
  (:`Pressed`
    (set `self.LoopCounter` 0)
    (if (not (== (`self.LoopCounter`) 3))
      (bind _rng_result (`self.RNG`))
      (set `self.Result_1` _rng_result)
      (`|ExecutionSequence`
        (:`then_0`
          (set `self.LoopCounter` 0)
          (bind _result (`/Engine/EditorBlueprintResources/StandardMacros.IncrementInt` (`self.LoopCounter`))
            (:`  `
              (set `self.LoopCounter` _result))))))))

(fn `RNG`
  (returns (RNG_Result :type Integer))
  (return (`KismetMathLibrary.RandomIntegerInRange` 0 (- (enumcount `/Game/Blueprints/GameLogic/E_WarChoices`) 1))))