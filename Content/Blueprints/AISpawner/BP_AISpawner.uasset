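; BP_AISpawner spawns BP_NPC patients whenever the reception desk is free.
; A looping timer starts on BeginPlay, presumably driving SpawnPacient, which checks the BP_Reception actor's IsFree flag.
; When free, it marks reception busy, spawns an NPC at SpawnLocation and sends it to ReceptionPoint.
; An older counted, delay-based spawn loop remains in the graph but never runs.
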(event `self.ReceiveBeginPlay`
  (`KismetSystemLibrary.K2_SetTimerDelegate` (`|CreateDelegate` :!event `SpawnPacient`) 0.3 true))

(event `SpawnPacient`
  (bind _returnvalue (`GameplayStatics.GetActorOfClass` "/Game/Blueprints/Bed/BP_Reception.BP_Reception_C"))
  (if (`/Game/Blueprints/Bed/BP_Reception.IsFree?` _returnvalue)
    (set `/Game/Blueprints/Bed/BP_Reception.IsFree?` false _returnvalue)
    (bind _returnvalue_2 (`AIBlueprintHelperLibrary.SpawnAIFromClass` "/Game/Blueprints/AI/NPC/BP_NPC.BP_NPC_C" null (`self.K2_GetActorLocation` (`self.SpawnLocation`)) (struct) false null))
    (bind _asbp_npc (cast `/Game/Blueprints/AI/NPC/BP_NPC` _returnvalue_2))
    (`/Game/Blueprints/AI/NPC/BP_NPC.MoveTo` _asbp_npc (`self.ReceptionPoint`))))

(fn `UserConstructionScript`)